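; Deprecated main character Blueprint, named as such, whose only active logic is firing projectiles on player input.
; Pressing Fire spawns the projectile class above the capsule, offset by its scaled height plus a margin, oriented to the control rotation and owned by the character.
; A CanFire flag with a short Delay acts as a cooldown between shots.
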(event `InputAction|Fire`
  (params (Key :type "Key Structure"))
  (bind _capsulecomponent (`self.CapsuleComponent`))
  (:`Pressed`
    (if (`self.CanFire`)
      (`|SpawnActorFromClass` "/Game/Player/Son/Projectiles/Projectiles.Projectiles_C" (`KismetMathLibrary.MakeTransform` (+ (`SceneComponent.K2_GetComponentLocation` _capsulecomponent) (`KismetMathLibrary.MakeVector` 0.0 0.0 (+ (* (`CapsuleComponent.GetScaledCapsuleHalfHeight` _capsulecomponent) 2.0) 20.0))) (`self.GetControlRotation`)) "Undefined" "OverrideRootScale" self null)
      (set `self.CanFire` false)
      (`KismetSystemLibrary.Delay` 0.5)
      (set `self.CanFire` true))))

(fn `UserConstructionScript`)