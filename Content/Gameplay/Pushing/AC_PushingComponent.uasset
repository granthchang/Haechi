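; Actor component that lets the Beast character grab a pushable object and push or pull it along its facing direction.
; BeginPush attaches the character to the object, stops rotation toward movement, hides the HUD prompt and enables tick; EndPush reverses the attachment and tick.
; Each tick it accelerates or decelerates forward input, then moves the object only if box and capsule traces find both object and character clear.
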(event `self.ReceiveBeginPlay`
  (`self.SetComponentTickEnabled` false)
  (bind _ascharacter (cast `Character` (`self.GetOwner`)))
  (set `self.Character` _ascharacter))

(event `self.ReceiveTick`
  (params (DeltaSeconds :type "Float (single-precision)"))
  (`self.HandleMovementInput` DeltaSeconds))

(fn `BeginPush`
  (params (PushableObject :type "/Game/Gameplay/Pushing/BP_PushableObject Object Reference"))
  (bind _character (`self.Character`))
  (`self.CurrentPushableObject`
    (:`then`)
    (:`else`
      (bind _output_get (set `self.CurrentPushableObject` PushableObject))
      (`Actor.K2_AttachToActor` _character _output_get "None" "KeepWorld" "KeepWorld" "KeepWorld" true)
      (set `CharacterMovementComponent.bOrientRotationToMovement` false (`Character.CharacterMovement` _character))
      (`self.SetComponentTickEnabled` true)
      (bind _asbp_beast (cast `/Game/Player/Beast/BP_Beast` (`self.Character`)))
      (bind _hud (`/Game/Player/Beast/BP_Beast.HUD` _asbp_beast)
        (:`then`
          (`/Game/UI/WBP_HUD.SetShowPushPrompt` _hud false))
        (:`else`)))))

(fn `EndPush`
  (bind _character (`self.Character`))
  (`self.CurrentPushableObject`
    (:`then`
      (set `self.CurrentPushableObject` null)
      (`Actor.K2_DetachFromActor` _character "KeepWorld" "KeepWorld" "KeepWorld")
      (set `CharacterMovementComponent.bOrientRotationToMovement` true (`Character.CharacterMovement` _character))
      (`self.SetComponentTickEnabled` false)
      (set `self.ForwardMove` 0.0))
    (:`else`)))

(fn `GetDeltaLocation`
  (params (DeltaSecond :type "Float (double-precision)") (Forward :type "Float (double-precision)"))
  (returns (`Delta Location` :type "Vector Structure"))
  (return (* (`Actor.GetActorForwardVector` (`self.Character`)) (`local.DeltaSecond`) (`self.Speed`) (`local.Forward`))))

(fn `HandleMovementInput`
  (params (DeltaSeconds :type "Float (double-precision)"))
  (bind _maxspeed (`self.MaxSpeed`))
  (bind _character (`self.Character`))
  (bind _capsulecomponent (`Character.CapsuleComponent` _character))
  (bind _returnvalue (+ (`Actor.K2_GetActorLocation` _character) (`self.GetDeltaLocation` (`local.DeltaSeconds`) (`self.ForwardMove`))))
  (bind _returnvalue_2 (+ (`self.ForwardMove`) (* (`self.ForwardInput`) (`self.Acceleration`))))
  ;[0 0 0] Acceleration/deceleration - if the final movement is 0, don't do anything
  (bind _output_get (set `self.ForwardMove` (select `bool` (== (`self.ForwardInput`) 0.0) :`false` (select `bool` (< (`self.ForwardInput`) 0.0) :`false` (`KismetMathLibrary.FClamp` _returnvalue_2 0.0 _maxspeed) :`true` (`KismetMathLibrary.FClamp` _returnvalue_2 (* _maxspeed -1.0) 0.0)) :`true` (select `bool` (< (`self.ForwardMove`) 0.0) :`false` (`KismetMathLibrary.FClamp` (- (`self.ForwardMove`) (`self.Decelleration`))) :`true` (`KismetMathLibrary.FClamp` (+ (`self.ForwardMove`) (`self.Decelleration`)) -1.0 0.0)))))
  (if (not (`KismetMathLibrary.NearlyEqual_FloatFloat` _output_get))
    (bind _currentpushableobject (`self.CurrentPushableObject`)
      (:`then`
        ;[0 0 0] Check that the object won't colide with anything
        (bind _asbp_beast (cast `/Game/Player/Beast/BP_Beast` (`self.Character`)))
        (bind (_origin _boxextent) (`KismetSystemLibrary.GetComponentBounds` (`/Game/Gameplay/Pushing/BP_PushableObject.StaticMesh` _currentpushableobject)))
        (bind _returnvalue_3 (+ (`self.GetDeltaLocation` (`local.DeltaSeconds`) (`self.ForwardMove`)) _origin))
        (bind (_outhit _returnvalue_4) (`KismetSystemLibrary.BoxTraceSingle` _returnvalue_3 _returnvalue_3 _boxextent (struct) "TraceTypeQuery1" false (`|MakeArray` (`self.CurrentPushableObject`) (`self.Character`) (`/Game/Player/Beast/BP_Beast.Player` _asbp_beast) :!type "Actor Object Reference")))
        (if _returnvalue_4
          (set `self.ForwardMove` 0.0)
          (else
            ;[0 0 0] Check that the player won't run into anything
            (bind _asbp_beast_2 (cast `/Game/Player/Beast/BP_Beast` (`self.Character`)))
            (bind (_outhit_2 _returnvalue_5) (`KismetSystemLibrary.CapsuleTraceSingle` _returnvalue _returnvalue (`CapsuleComponent.GetScaledCapsuleRadius` _capsulecomponent) (`CapsuleComponent.GetScaledCapsuleHalfHeight` _capsulecomponent) "TraceTypeQuery1" false (`|MakeArray` (`self.CurrentPushableObject`) (`self.Character`) (`/Game/Player/Beast/BP_Beast.Player` _asbp_beast_2) :!type "Actor Object Reference") "None" true (struct :`R` 1.0 :`A` 1.0) (struct :`G` 1.0 :`A` 1.0) 1.0))
            (if _returnvalue_5
              (set `self.ForwardMove` 0.0)
              (else
                ;[0 0 0] Move
                (`Actor.K2_AddActorWorldOffset` (`self.CurrentPushableObject`) (`self.GetDeltaLocation` (`local.DeltaSeconds`) (`self.ForwardMove`)) false false))))))
      (:`else`))))

(fn `IsHoldingObject`
  (returns (`Return Value` :type Boolean))
  (return (`KismetSystemLibrary.IsValid` (`self.CurrentPushableObject`))))