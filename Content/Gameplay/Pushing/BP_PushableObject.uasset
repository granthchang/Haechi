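; BP_PushableObject is an actor that characters with an AC_PushingComponent can push from predefined sides, stored as PushDirections transforms and shown as arrows.
; Hold selects the side nearest the character within the component's range, then validates that spot with capsule and line traces for room, walkable floor and obstructions.
; A timeline moves the player into place, then calls BeginPush if BP_Player still has the push key pressed.
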(event `/Game/Gameplay/Pushing/BPI_Pushable.Hold`
  (params (Character :type "/Game/Player/Son/BP_Player Object Reference"))
  (bind _returnvalue (`self.GetComponentByClass` Character "/Game/Gameplay/Pushing/AC_PushingComponent.AC_PushingComponent_C"))
  ;[0 0 0] Ensure this character is a valid pushing character
  (`/Engine/EditorBlueprintResources/StandardMacros.IsValid` Character
    (:`Is Valid`
      (`/Engine/EditorBlueprintResources/StandardMacros.IsValid` _returnvalue
        (:`Is Valid`
          (set `self.Player` Character)
          (bind _output_get (set `self.Pushing Component` _returnvalue))
          ;[0 0 0] Find which side to go to
          (bind _index (`self.GetClosestPushDirectionIndex` (`KismetMathLibrary.Conv_VectorToVector2D` (`self.K2_GetActorLocation` (`self.Player`))) (`/Game/Gameplay/Pushing/AC_PushingComponent.Range` _output_get)))
          (if (>= _index 0)
            ;[0 0 0] Find new character location
            (bind (_locationisvalid _newlocation) (`self.TryGetNewLocation` _index))
            (if _locationisvalid
              ;[0 0 0] Smoothly move player to new location
              (bind (_direction _alpha) (`Timeline|Go to next location` :!via `PlayFromStart`)
                (:`Update`
                  (`self.K2_SetActorTransform` (`self.Player`) (`KismetMathLibrary.TLerp` (`self.GetTransform` (`self.Player`)) _newlocation _alpha) false false))
                (:`Finished`
                  ;[0 0 0] Start pushing once the player is at the new location
                  (bind _asbp_player (cast `/Game/Player/Son/BP_Player` (`self.Player`)))
                  (if (`/Game/Player/Son/BP_Player.IsPushKeyPressed` _asbp_player)
                    (`/Game/Gameplay/Pushing/AC_PushingComponent.BeginPush` (`self.Pushing Component`) self)))))))))))

(fn `GetClosestPushDirectionIndex`
  (params (`Character Location` :type "Vector2D Structure") (Range :type "Float (double-precision)"))
  (returns (Index :type Integer))
  (locals (`Current Index` :type Integer) (`Current Distance Sq` :type "Float (double-precision)" :default 0.0) (`Closest Index` :type Integer :default -1) (`Closest Distance Sq` :type "Float (double-precision)"))
  (for (_array_element _array_index) (`self.PushDirections`)
    (set `local.Current Index` _array_index)
    (set `local.Current Distance Sq` (`KismetMathLibrary.DistanceSquared2D` (`KismetMathLibrary.Conv_VectorToVector2D` (`KismetMathLibrary.TransformLocation` (`self.GetTransform`) (.location _array_element))) (`local.Character Location`)))
    (if (and (< (`local.Current Distance Sq`) (`KismetMathLibrary.Square` (`local.Range`))) (or (< (`local.Current Distance Sq`) (`local.Closest Distance Sq`)) (< (`local.Closest Index`) 0)))
      (set `local.Closest Index` (`local.Current Index`))
      (set `local.Closest Distance Sq` (`local.Current Distance Sq`))))
  (return (`local.Closest Index`)))

(fn `TryGetNewLocation`
  (params (Index :type Integer))
  (returns (LocationIsValid :type Boolean) (NewLocation :type "Transform Structure"))
  (locals (NewCharacterLocation :type "Transform Structure"))
  (bind _newcharacterlocation_location (`KismetMathLibrary.BreakTransform` (`local.NewCharacterLocation`)))
  (bind _newcharacterlocation_location_2 (`KismetMathLibrary.BreakTransform` (`local.NewCharacterLocation`)))
  (bind (_returnvalue_location _returnvalue_rotation _returnvalue_scale) (`KismetMathLibrary.BreakTransform` (`self.GetTransform` (`self.Player`))))
  (bind _capsulecomponent (`Character.CapsuleComponent` (`self.Player`)))
  (bind (_returnvalue_location_2 _returnvalue_rotation_2) (`KismetMathLibrary.BreakTransform` (`KismetMathLibrary.ComposeTransforms` (`|GetArrayItem` (`self.PushDirections`) Index) (`self.GetTransform`))))
  ;[0 0 0] Check that the new Character location is valid
  ; - Has room to stand
  ; - On walkable floor
  (set `local.NewCharacterLocation` (`KismetMathLibrary.MakeTransform` (+ _returnvalue_location_2 (`KismetMathLibrary.MakeVector` 0.0 0.0 (`CapsuleComponent.GetScaledCapsuleHalfHeight` (`Character.CapsuleComponent` (`self.Player`))))) _returnvalue_rotation_2 _returnvalue_scale))
  (bind _outhit (`KismetSystemLibrary.CapsuleTraceSingle` (+ (0.0 0.0 20.0) _newcharacterlocation_location) (- _newcharacterlocation_location (0.0 0.0 20.0)) (`CapsuleComponent.GetScaledCapsuleRadius` _capsulecomponent) (`CapsuleComponent.GetScaledCapsuleHalfHeight` _capsulecomponent) "TraceTypeQuery1" false (`|MakeArray` (`self.Player`) :!type "Actor Object Reference") "None" true (struct :`R` 1.0 :`A` 1.0) (struct :`G` 1.0 :`A` 1.0) 1.0))
  (if (not (`.bInitialOverlap` (`GameplayStatics.BreakHitResult` _outhit)))
    (if (< (`CharacterMovementComponent.K2_GetWalkableFloorZ` (`Character.CharacterMovement` (`self.Player`))) (.z (`.ImpactNormal` (`GameplayStatics.BreakHitResult` _outhit))))
      ;[0 0 0] Check that nothing is between current and new Character location
      (bind (_outhits _returnvalue) (`KismetSystemLibrary.LineTraceMulti` (`self.K2_GetActorLocation`) _newcharacterlocation_location_2 "TraceTypeQuery1" false (`|MakeArray` (`self.Player`) :!type "Actor Object Reference") "None" true (struct :`R` 1.0 :`A` 1.0) (struct :`G` 1.0 :`A` 1.0) 0.5))
      (if (not _returnvalue)
        (return true (`local.NewCharacterLocation`))
        (else
          (`KismetSystemLibrary.PrintString` "WallsBetween character and object")
          (return false)))
      (else
        (`KismetSystemLibrary.PrintString` "floor not walkable")
        (return false)))
    (else
      (`KismetSystemLibrary.PrintString` "no room to stand")
      (return false))))

(fn `UserConstructionScript`
  (`StaticMeshComponent.SetStaticMesh` (`self.StaticMesh`) (`self.Mesh`))
  (for _array_element (`self.PushDirections`)
    (`AddComponent|NODE_AddArrowComponent-0` :`RelativeTransform` _array_element)))