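; Actor component that lets its owning Character push and drag BP_MovableObject actors.
; While not pushing, Tick traces a short line forward on the Visibility channel, caches any movable object hit and toggles the push prompt on WBP_HUD.
; OnBeginPush attaches the cached object to the Character with world transform kept, and OnEndPush detaches it.
; The HUD reference comes from the first top-level WBP_HUD found at BeginPlay.
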(event `self.ReceiveBeginPlay`
  (bind _ascharacter (cast `Character` (`self.GetOwner`)))
  (set `self.Character` _ascharacter)
  (bind _foundwidgets (`WidgetBlueprintLibrary.GetAllWidgetsOfClass` "/Game/UI/WBP_HUD.WBP_HUD_C"))
  (set `self.WBP HUD` (`|GetArrayItem` _foundwidgets)))

(event `self.ReceiveTick`
  (params (DeltaSeconds :type "Float (single-precision)"))
  (bind _character (`self.Character`))
  (bind _returnvalue (`Actor.K2_GetActorLocation` _character))
  (if (not (`self.IsPushing`))
    (bind (_outhit _returnvalue_2) (`KismetSystemLibrary.LineTraceSingle` :`Start` _returnvalue :`End` (+ _returnvalue (* 150.0 (`Actor.GetActorForwardVector` _character))) :`TraceChannel` "TraceTypeQuery1" :`DrawTime` 1.0))
    (if _returnvalue_2
      (bind _asbp_movable_object (cast `/Game/Gameplay/BP_MovableObject` (`.HitActor` (`GameplayStatics.BreakHitResult` _outhit)))
        (:`then`
          (set `self.PushableObject` _asbp_movable_object)
          (`/Game/UI/WBP_HUD.SetShowPushPrompt` (`self.WBP HUD`) true))
        (:`CastFailed`
          (set `self.PushableObject` null :!label _label)
          (`/Game/UI/WBP_HUD.SetShowPushPrompt` (`self.WBP HUD`) false)))
      (else
        (goto _label)))))

(event `OnBeginPush`
  (bind _pushableobject (`self.PushableObject`)
    (:`then`
      (`Actor.K2_AttachToActor` _pushableobject (`self.Character`) "None" "KeepWorld" "KeepWorld" "KeepWorld" true)
      (set `self.IsPushing` true))
    (:`else`)))

(event `OnEndPush`
  (bind _pushableobject (`self.PushableObject`)
    (:`then`
      (`Actor.K2_DetachFromActor` _pushableobject "KeepWorld" "KeepWorld" "KeepWorld")
      (set `self.IsPushing` false))
    (:`else`)))